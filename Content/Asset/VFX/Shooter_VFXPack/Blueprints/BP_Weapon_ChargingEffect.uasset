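; Weapon charging-effect actor that automatically loops a Niagara charge-up on a first-person gun attached to the arm mesh's grip socket, likely as a VFX showcase.
; After an initial delay, each cycle restarts the effect, and a FlipFlop alternates between cancelling the charge and firing.
; Firing waits through one of two alternating charge durations, spawns BP_Projectile_Big at the arrow with configurable effects, plays the fire montage, then repeats.
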(event `Again`
  (bind _chargingeffect (`self.ChargingEffect`))
  (`KismetSystemLibrary.Delay` (`self.Delay`))
  (`NiagaraComponent.SetAsset` (`self.ChargingEffect`) (`self.MuzzleFlash_Effect`) true :!label _label)
  (`ActorComponent.Activate` _chargingeffect true)
  (`/Engine/EditorBlueprintResources/StandardMacros.FlipFlop`
    (:`A`
      (`KismetSystemLibrary.Delay` 1.75)
      (`ActorComponent.Deactivate` _chargingeffect)
      (`self.Again`))
    (:`B`
      (`/Engine/EditorBlueprintResources/StandardMacros.FlipFlop`
        (:`A`
          (`KismetSystemLibrary.Delay` 5.0))
        (:`B`
          (`KismetSystemLibrary.Delay` 2.5)))
      (`|SpawnActorFromClass` "/Game/Asset/VFX/Shooter_VFXPack/Blueprints/BP_Projectile_Big.BP_Projectile_Big_C" (`SceneComponent.K2_GetComponentToWorld` (`self.Arrow`)) "Undefined" "OverrideRootScale" null (`self.Initial Speed`) (`self.bGravity Enabled`) (`self.Niagara_Trail`) (`self.Niagara_Hit`) (`self.bMuzzleFlashAndHit`) (`self.bImpact Normal`) (`self.Niagara_Projectile`) (`self.DecalEmissive Color`) null)
      (`AnimInstance.Montage_Play` (`SkeletalMeshComponent.GetAnimInstance` (`self.SkeletalMesh`)) "/Game/Asset/VFX/Shooter_VFXPack/DEMO/Character_02/Animations/FirstPersonFire_Montage.FirstPersonFire_Montage" 1.0 "MontageLength" 0.0 true) ; Play animation on arm mesh
      (`ActorComponent.Deactivate` (`self.ChargingEffect`))
      (`self.Again`))))

(event `self.ReceiveBeginPlay`
  (`KismetSystemLibrary.Delay` (`self.InitialDelay`))
  (goto _label))

(fn `UserConstructionScript`
  (`SceneComponent.K2_AttachToComponent` (`self.FP_Gun`) (`self.SkeletalMesh`) "GripPoint" "SnapToTarget" "SnapToTarget" "SnapToTarget" true))
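; BP_ES_HUD is the gameplay HUD that creates the main UI and exposes functions for warehouse, shop, interaction prompts and item tooltips.
; On BeginPlay it spawns WBP_Gameplay_Main, caches its panels and adds a hidden high Z-order tooltip.
; Panel and interaction functions forward to those widgets, with warehouse and shop opening alongside the inventory.
; Tick moves the visible tooltip to the mouse, clamped inside the DPI-scaled viewport's right and bottom edges.
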(event `self.ReceiveBeginPlay`
  (`|ExecutionSequence`
    (:`then_0`
      (bind _returnvalue (`|CreateWidget` "/Game/Blueprint/UI/Main/WBP_Gameplay_Main.WBP_Gameplay_Main_C"))
      (bind _output_get (set `self.Ref_Main` _returnvalue))
      (`UserWidget.AddToViewport` _output_get 0)
      (set `self.CachedWarehousePanel` (`/Game/Blueprint/UI/Main/WBP_Gameplay_Main.WBP_ES_WarehousePanel` (`self.Ref_Main`)))
      (set `self.CachedInventoryMain` (`/Game/Blueprint/UI/Main/WBP_Gameplay_Main.WBP_ES_InventoryMain` (`self.Ref_Main`)))
      (set `self.CachedShopPanel` (`/Game/Blueprint/UI/Main/WBP_Gameplay_Main.WBP_ES_ShopPanel` (`self.Ref_Main`))))
    (:`then_1`
      (bind _returnvalue_2 (`|CreateWidget` (`self.TooltipWidgetClass`)))
      (set `self.CachedTooltip` _returnvalue_2)
      (`UserWidget.AddToViewport` (`self.CachedTooltip`) 100)
      (`Widget.SetVisibility` (`self.CachedTooltip`) "Hidden"))))

(event `self.ReceiveTick`
  (params (DeltaSeconds :type "Float (single-precision)"))
  (`|ExecutionSequence`
    (:`then_0`
      (`self.UpdateTooltipPosition`))))

(fn `ChangeInteractionVisibility`
  (params (IsAdd :type Boolean) (InText :type Text) (TextColor :type "LinearColor Structure" :default (struct :`R` 1.0 :`G` 1.0 :`B` 1.0 :`A` 1.0)) (InteractionActor :type "Actor Object Reference"))
  (if IsAdd
    (`/Game/Blueprint/UI/Main/WBP_Gameplay_Main.AddInteractionUI` (`self.Ref_Main`) InText TextColor false InteractionActor)
    (else
      (`/Game/Blueprint/UI/Main/WBP_Gameplay_Main.RemoveInteractionUI` (`self.Ref_Main`) InteractionActor))))

(fn `CloseShopPanel`
  (`/Game/Blueprint/Item/UI/Shop/WBP_ES_ShopPanel.CloseShop` (`self.CachedShopPanel`)))

(fn `CloseWarehousePanel`
  (`/Game/Blueprint/Item/UI/Warehouse/WBP_ES_WarehousePanel.CloseWarehouse` (`self.CachedWarehousePanel`)))

(fn `HideTooltip`
  (`Widget.SetVisibility` (`self.CachedTooltip`) "Hidden"))

(fn `OpenShopPanel`
  (`Widget.SetVisibility` (`self.CachedInventoryMain`) "SelfHitTestInvisible")
  (`Widget.SetVisibility` (`self.CachedShopPanel`) "SelfHitTestInvisible"))

(fn `OpenWarehousePanel`
  (`Widget.SetVisibility` (`self.CachedWarehousePanel`) "SelfHitTestInvisible")
  (`Widget.SetVisibility` (`self.CachedInventoryMain`) "SelfHitTestInvisible"))

(fn `ShowTooltip`
  (params (EquipItem :type "ESEquipItemBase Object Reference"))
  (`/Game/Blueprint/Item/UI/Tooltip/WBP_ES_ItemTooltip.SetTooltipData` (`self.CachedTooltip`) EquipItem)
  (`Widget.SetVisibility` (`self.CachedTooltip`) "HitTestInvisible"))

(fn `SwitchInteractionMenu`
  (params (bIsNext :type Boolean))
  (`/Game/Blueprint/UI/Main/WBP_Gameplay_Main.ChangeInteractionUI` (`self.Ref_Main`) bIsNext))

(fn `TriggerInteractionActor`
  (`/Game/Blueprint/UI/Main/WBP_Gameplay_Main.TriggerInteractionUI` (`self.Ref_Main`)))

(fn `UpdateTooltipPosition`
  (locals (MouseXY :type "Vector2D Structure") (TooltipWH :type "Vector2D Structure") (ViewportWH :type "Vector2D Structure"))
  (bind (_x _y) (`KismetMathLibrary.BreakVector2D` (`Widget.GetDesiredSize` (`self.CachedTooltip`))))
  (bind (_x_2 _y_2) (`KismetMathLibrary.BreakVector2D` (/ (`WidgetLayoutLibrary.GetViewportSize`) (`WidgetLayoutLibrary.GetViewportScale`))))
  (`/Engine/EditorBlueprintResources/StandardMacros.IsValid` (`self.CachedTooltip`)
    (:`Is Valid`
      (if (`Widget.IsVisible` (`self.CachedTooltip`))
        (bind _returnvalue (`WidgetLayoutLibrary.GetMousePositionOnViewport`))
        (bind (_x_3 _y_3) (`KismetMathLibrary.BreakVector2D` _returnvalue))
        (`UserWidget.SetPositionInViewport` (`self.CachedTooltip`) (`KismetMathLibrary.MakeVector2D` (`KismetMathLibrary.FMin` _x_3 (- _x_2 _x)) (`KismetMathLibrary.FMin` _y_3 (- _y_2 _y))) false)))))

(fn `UserConstructionScript`)
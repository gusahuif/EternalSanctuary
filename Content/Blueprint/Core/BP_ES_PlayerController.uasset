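; Player controller that routes Enhanced Input actions for inventory and interaction to the ES HUD.
; The inventory action toggles the HUD's cached main inventory widget between hidden and visible without blocking hit tests on its children.
; The interaction action triggers the HUD's interaction actor, and the mouse wheel's sign sets the direction for switching the interaction menu.
; Level-loading and input-mode nodes are present but unconnected.
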(event `self.ReceiveBeginPlay`)

(event `EnhancedInput|/Game/Input/Gameplay/InputAction/IA_Inventory`
  (params (ActionValue :type Boolean) (ElapsedSeconds :type "Float (double-precision)") (TriggeredSeconds :type "Float (double-precision)") (InputAction :type "InputAction Object Reference" :default "/Game/Input/Gameplay/InputAction/IA_Inventory.IA_Inventory"))
  (bind _cachedinventorymain (`/Game/Blueprint/Core/BP_ES_HUD.CachedInventoryMain` (`/Game/Blueprint/Item/Lib/BFL_Item.GetESHUD`)))
  (:`Started`
    (if (`Widget.IsVisible` _cachedinventorymain)
      (`Widget.SetVisibility` _cachedinventorymain "Hidden")
      (else
        (`Widget.SetVisibility` _cachedinventorymain "SelfHitTestInvisible")))))

(event `EnhancedInput|/Game/Input/Gameplay/InputAction/IA_Interaction`
  (params (ActionValue :type Boolean) (ElapsedSeconds :type "Float (double-precision)") (TriggeredSeconds :type "Float (double-precision)") (InputAction :type "InputAction Object Reference" :default "/Game/Input/Gameplay/InputAction/IA_Interaction.IA_Interaction"))
  (:`Started`
    (`/Game/Blueprint/Core/BP_ES_HUD.TriggerInteractionActor` (`/Game/Blueprint/Item/Lib/BFL_Item.GetESHUD`))))

(event `EnhancedInput|/Game/Input/Gameplay/InputAction/IA_MouseWheel`
  (params (ActionValue :type "Float (double-precision)") (ElapsedSeconds :type "Float (double-precision)") (TriggeredSeconds :type "Float (double-precision)") (InputAction :type "InputAction Object Reference" :default "/Game/Input/Gameplay/InputAction/IA_MouseWheel.IA_MouseWheel"))
  (:`Started`
    (`/Game/Blueprint/Core/BP_ES_HUD.SwitchInteractionMenu` (`/Game/Blueprint/Item/Lib/BFL_Item.GetESHUD`) (> ActionValue 0.0))))

(fn `UserConstructionScript`)
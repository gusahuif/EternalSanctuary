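; Area-of-effect actor for the Archer's Arrow Storm skill that damages and slows enemies inside it.
; Sphere overlaps maintain an enemy list, applying the slow effect on entry and removing active effects by skill tag on exit.
; Each Tick sends GE_Damage from the owner's ability system to listed enemies, with a negative SetByCaller bonus.
; After a few seconds it stops Niagara and overlap generation, then destroys itself shortly after.
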(event `self.ReceiveBeginPlay`
  (`KismetSystemLibrary.Delay` 3.0)
  (`ActorComponent.Deactivate` (`self.Niagara`))
  (set `PrimitiveComponent.bGenerateOverlapEvents` false (`self.Sphere`))
  (`KismetSystemLibrary.Delay` 1.0)
  (`self.K2_DestroyActor`))

(event `self.ReceiveTick`
  (params (DeltaSeconds :type "Float (single-precision)"))
  (bind _enemylist (`self.EnemyList`))
  (bind _returnvalue (`AbilitySystemBlueprintLibrary.GetAbilitySystemComponent` (`self.GetOwner`)))
  (if (> (`KismetArrayLibrary.Array_Length` _enemylist) 0)
    (for _array_element _enemylist
      (bind _returnvalue_2 (`AbilitySystemBlueprintLibrary.AssignTagSetByCallerMagnitude` (`AbilitySystemComponent.MakeOutgoingSpec` _returnvalue "/Game/Blueprint/GAS/GameplayEffect/Combat/GE_Damage.GE_Damage_C" 0.0 (`AbilitySystemComponent.MakeEffectContext` _returnvalue)) (struct :`TagName` "Damage.AbilityTypeBonus") -0.6))
      (`AbilitySystemComponent.BP_ApplyGameplayEffectSpecToTarget` _returnvalue _returnvalue_2 (`ESCharacterBase.GetESAbilitySystemComponent` _array_element)))))

(event `self.Sphere.OnComponentBeginOverlap`
  (params (OverlappedComponent :type "PrimitiveComponent Object Reference") (OtherActor :type "Actor Object Reference") (OtherComp :type "PrimitiveComponent Object Reference") (OtherBodyIndex :type Integer) (bFromSweep :type Boolean) (SweepResult :type "HitResult Structure (by ref)"))
  (bind _returnvalue (`AbilitySystemBlueprintLibrary.GetAbilitySystemComponent` (`self.GetOwner`)))
  (bind _asbp_enemy_base (cast `/Game/Blueprint/Character/Enemy/BP_EnemyBase` OtherActor))
  (if (not (`KismetArrayLibrary.Array_Contains` (`self.EnemyList`) _asbp_enemy_base))
    (`KismetArrayLibrary.Array_Add` (`self.EnemyList`) _asbp_enemy_base)
    (`AbilitySystemComponent.BP_ApplyGameplayEffectToTarget` _returnvalue "/Game/Blueprint/GAS/GameplayAbility/Archer/ArrowStorm/Skill/GE_Archer_ArrowStorm_Slow.GE_Archer_ArrowStorm_Slow_C" (`ESCharacterBase.GetESAbilitySystemComponent` _asbp_enemy_base) 0.0 (`AbilitySystemComponent.MakeEffectContext` _returnvalue))))

(event `self.Sphere.OnComponentEndOverlap`
  (params (OverlappedComponent :type "PrimitiveComponent Object Reference") (OtherActor :type "Actor Object Reference") (OtherComp :type "PrimitiveComponent Object Reference") (OtherBodyIndex :type Integer))
  (bind _enemylist (`self.EnemyList`))
  (bind _asbp_enemy_base (cast `/Game/Blueprint/Character/Enemy/BP_EnemyBase` OtherActor))
  (if (`KismetArrayLibrary.Array_Contains` _enemylist _asbp_enemy_base)
    (`KismetArrayLibrary.Array_RemoveItem` _enemylist _asbp_enemy_base)
    (`AbilitySystemComponent.RemoveActiveEffectsWithTags` (`AbilitySystemBlueprintLibrary.GetAbilitySystemComponent` _asbp_enemy_base) (struct :`GameplayTags` (struct :`(TagName` "Ability.Archer.ArrowStorm.Skill"))))))

(fn `UserConstructionScript`)
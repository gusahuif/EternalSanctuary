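; Archer charge-and-release gameplay ability that fires a piercing shot scaled by how long it is held.
; Activation begins a cast, plays the bow start montage, enables rotation updates and raises a capped charge counter through a looping Delay.
; On key release, a confirmed charge spawns the projectile at the left hand with charge-based penetration and ability bonus, locks rotation and jumps to the Finish section.
; An unconfirmed charge or montage end ends the ability.
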(event `self.K2_ActivateAbility`
  (bind _returnvalue (`self.GetESOwnerCharacter`))
  (set `self.ChargedCount` 0)
  (`ESPlayerBase.BeginCast` _returnvalue false)
  (`ESPlayerBase.ChangeCommandState` _returnvalue "Cast")
  (`AbilityTask_PlayMontageAndWait.CreatePlayMontageAndWaitProxy` "None" "/Game/Blueprint/GAS/GameplayAbility/Archer/ChargedPiercingShot/Anim/GhostSamurai_Bow_Shoot_SP_Start_Root_Montage.GhostSamurai_Bow_Shoot_SP_Start_Root_Montage"
    (:`then`
      (`|ExecutionSequence`
        (:`then_0`
          (`KismetSystemLibrary.Delay` 0.2 :!label _label)
          (bind _result (`/Engine/EditorBlueprintResources/StandardMacros.IncrementInt` (`self.ChargedCount`))
            (:`  `
              (if (not (>= _result 4))
                (goto _label)))))
        (:`then_1`
          (bind _asbp_es_player_base (cast `/Game/Blueprint/Character/Player/BP_ES_PlayerBase` (`self.GetESOwnerCharacter`)))
          (set `/Game/Blueprint/Character/Player/BP_ES_PlayerBase.bCanUpdateRotation` true _asbp_es_player_base))))
    (:`OnCompleted`
      (`self.K2_EndAbility` :!label _label_2))
    (:`OnInterrupted`
      (goto _label_2))
    (:`OnCancelled`
      (goto _label_2))))

(event `self.OnSkillKeyboardRelease`
  (bind _chargedcount (`self.ChargedCount`))
  (`parent.OnSkillKeyboardRelease`)
  (bind _returnvalue (`self.ServerConfirmCharge`))
  (if _returnvalue
    (bind _ascharacter (cast `Character` (`self.GetAvatarActorFromActorInfo`)))
    (`|SpawnActorFromClass` "/Game/Blueprint/GAS/GameplayAbility/Archer/ChargedPiercingShot/Projectile/BP_ChargedPiercingShot.BP_ChargedPiercingShot_C" (`KismetMathLibrary.MakeTransform` (`SceneComponent.GetSocketLocation` (`Character.Mesh` _ascharacter) "hand_l") (`Actor.K2_GetActorRotation` _ascharacter)) "AlwaysSpawn" "MultiplyWithRoot" _ascharacter _chargedcount 2000.0 2000.0 (- (+ (* (`KismetMathLibrary.Conv_IntToDouble` _chargedcount) 0.2) 0.8) 1.0) _ascharacter)
    (bind _asbp_es_player_base (cast `/Game/Blueprint/Character/Player/BP_ES_PlayerBase` (`self.GetESOwnerCharacter`)))
    (set `/Game/Blueprint/Character/Player/BP_ES_PlayerBase.bCanUpdateRotation` false _asbp_es_player_base)
    (`self.MontageJumpToSection` "Finish")
    (else
      (`self.K2_EndAbility`))))
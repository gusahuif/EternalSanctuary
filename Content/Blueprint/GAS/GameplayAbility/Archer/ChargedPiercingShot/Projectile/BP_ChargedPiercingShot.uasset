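; Projectile Blueprint for the Archer's Charged Piercing Shot ability, leaving collision handling to its parent class.
; On delayed destroy it calls the parent, then deactivates its rainbow trail effect.
; Disconnected, never-executed nodes hold owner ability-system caching and Archer rune logic: Gale stacking, Pierce vulnerability, and Hunt damage scaled by the remaining Mark duration, which consumes the Mark.
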(event `self.ReceiveBeginPlay`
  (`parent.ReceiveBeginPlay`))

(event `self.HandleProjectileCollision`
  (params (OtherActor :type "Actor Object Reference") (OtherComp :type "PrimitiveComponent Object Reference") (bFromSweep :type Boolean) (SweepResult :type "HitResult Structure (by ref)"))
  (`parent.HandleProjectileCollision` OtherActor OtherComp bFromSweep SweepResult))

(event `self.BlueprintDelayedDestroy`
  (`parent.BlueprintDelayedDestroy`)
  (`ActorComponent.Deactivate` (`self.P_Trail_Rainbow`)))

(fn `UserConstructionScript`
  (`parent.UserConstructionScript`))
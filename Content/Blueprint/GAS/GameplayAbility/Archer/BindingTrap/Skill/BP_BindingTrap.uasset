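; Archer Binding Trap actor that detonates when an enemy enters its trigger sphere, damaging enemies in its area.
; SphereDamage overlap events keep a list of the enemies currently inside that radius.
; On trigger, the owner's Ability System Component applies GE_Damage to each listed enemy, using a SetByCaller ability-type bonus.
; The trap then fires its hit GameplayCue at its location and destroys itself.
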(event `self.SphereTrigger.OnComponentBeginOverlap`
  (params (OverlappedComponent :type "PrimitiveComponent Object Reference") (OtherActor :type "Actor Object Reference") (OtherComp :type "PrimitiveComponent Object Reference") (OtherBodyIndex :type Integer) (bFromSweep :type Boolean) (SweepResult :type "HitResult Structure (by ref)"))
  (bind _returnvalue (`AbilitySystemBlueprintLibrary.GetAbilitySystemComponent` (`self.GetOwner`)))
  (cast `/Game/Blueprint/Character/Enemy/BP_EnemyBase` OtherActor)
  (for _array_element (`self.EnemyList`)
    (bind _returnvalue_2 (`AbilitySystemBlueprintLibrary.AssignTagSetByCallerMagnitude` (`AbilitySystemComponent.MakeOutgoingSpec` _returnvalue "/Game/Blueprint/GAS/GameplayEffect/Combat/GE_Damage.GE_Damage_C" 0.0 (`AbilitySystemComponent.MakeEffectContext` _returnvalue)) (struct :`TagName` "Damage.AbilityTypeBonus") 0.1))
    (`AbilitySystemComponent.BP_ApplyGameplayEffectSpecToTarget` _returnvalue _returnvalue_2 (`AbilitySystemBlueprintLibrary.GetAbilitySystemComponent` _array_element)))
  (`GameplayCueFunctionLibrary.ExecuteGameplayCueOnActor` self (struct :`TagName` "GameplayCue.Hit.Archer.BindingTrap") (`AbilitySystemBlueprintLibrary.MakeGameplayCueParameters` 0.0 0.0 (struct) (struct) (struct) (struct) (struct) (`self.K2_GetActorLocation`)))
  (`self.K2_DestroyActor`))

(event `self.SphereDamage.OnComponentBeginOverlap`
  (params (OverlappedComponent :type "PrimitiveComponent Object Reference") (OtherActor :type "Actor Object Reference") (OtherComp :type "PrimitiveComponent Object Reference") (OtherBodyIndex :type Integer) (bFromSweep :type Boolean) (SweepResult :type "HitResult Structure (by ref)"))
  (bind _asbp_enemy_base (cast `/Game/Blueprint/Character/Enemy/BP_EnemyBase` OtherActor))
  (`KismetArrayLibrary.Array_AddUnique` (`self.EnemyList`) _asbp_enemy_base))

(event `self.SphereDamage.OnComponentEndOverlap`
  (params (OverlappedComponent :type "PrimitiveComponent Object Reference") (OtherActor :type "Actor Object Reference") (OtherComp :type "PrimitiveComponent Object Reference") (OtherBodyIndex :type Integer))
  (bind _asbp_enemy_base (cast `/Game/Blueprint/Character/Enemy/BP_EnemyBase` OtherActor))
  (`KismetArrayLibrary.Array_RemoveItem` (`self.EnemyList`) _asbp_enemy_base))

(fn `UserConstructionScript`)
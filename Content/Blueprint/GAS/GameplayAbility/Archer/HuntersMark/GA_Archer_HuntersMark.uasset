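; Archer Hunter's Mark gameplay ability that marks the owner's current attack target, ending at once if there is no valid target.
; It applies the Hunter's Mark gameplay effect to that enemy and adds a gameplay cue on it, with the avatar as instigator.
; The ability stays active until a fixed delay expires or a watched attribute on the enemy drops to zero or below, then ends.
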(event `self.K2_ActivateAbility`
  (bind _returnvalue (`self.GetESAbilitySystemComponent`))
  (bind _returnvalue_2 (`ESPlayerBase.GetAttackTarget` (`self.GetESOwnerCharacter`)))
  (`/Engine/EditorBlueprintResources/StandardMacros.IsValid` _returnvalue_2
    (:`Is Valid`
      (set `self.Ref_Enemy` _returnvalue_2)
      (`AbilitySystemComponent.BP_ApplyGameplayEffectToTarget` _returnvalue "/Game/Blueprint/GAS/GameplayAbility/Archer/HuntersMark/Effect/GE_Archer_HuntersMark.GE_Archer_HuntersMark_C" (`AbilitySystemBlueprintLibrary.GetAbilitySystemComponent` (`self.Ref_Enemy`)) 0.0 (`AbilitySystemComponent.MakeEffectContext` _returnvalue))
      (`GameplayCueFunctionLibrary.AddGameplayCueOnActor` (`self.Ref_Enemy`) (struct :`TagName` "GameplayCue.Skill.Archer.HuntesMark") (`AbilitySystemBlueprintLibrary.MakeGameplayCueParameters` 0.0 0.0 (struct) (struct) (struct) (struct) (struct) (0.0 0.0 0.0) (0.0 0.0 0.0) (`self.GetAvatarActorFromActorInfo`)))
      (bind (_asynctaskproxy _attribute _newvalue) (`AbilityAsync_WaitAttributeChanged.WaitForAttributeChanged` (`self.Ref_Enemy`) (struct :`AttributeName` "Health" :`Attribute` "/Script/EternalSanctuary.ESAttributeSet:Health" :`AttributeOwner` "/Script/CoreUObject.Class'/Script/EternalSanctuary.ESAttributeSet'"))
        (:`then`
          (`KismetSystemLibrary.Delay` 8.0)
          (`self.K2_EndAbility` :!label _label))
        (:`Changed`
          (if (<= _newvalue 0.0)
            (goto _label)))))
    (:`Is Not Valid`
      (`self.K2_EndAbility`))))
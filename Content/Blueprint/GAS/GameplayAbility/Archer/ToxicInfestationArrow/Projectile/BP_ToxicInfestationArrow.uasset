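; Projectile for the Archer's Toxic Infestation Arrow ability, built on a parent projectile class.
; On collision it runs the parent handling, then applies the toxic infestation GameplayEffect from the owner's ASC to the hit actor, using a SetByCaller ability-type damage bonus.
; On delayed destroy it deactivates the poison trail.
; Owner-ASC setup and Gale, Pierce and Hunt rune logic are present but disconnected, so they never run.
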(event `self.ReceiveBeginPlay`
  (`parent.ReceiveBeginPlay`))

(event `self.HandleProjectileCollision`
  (params (OtherActor :type "Actor Object Reference") (OtherComp :type "PrimitiveComponent Object Reference") (bFromSweep :type Boolean) (SweepResult :type "HitResult Structure (by ref)"))
  (bind _ownerasc (`self.OwnerASC`))
  (`parent.HandleProjectileCollision` OtherActor OtherComp bFromSweep SweepResult)
  (bind _returnvalue (`AbilitySystemBlueprintLibrary.AssignTagSetByCallerMagnitude` (`AbilitySystemComponent.MakeOutgoingSpec` _ownerasc "/Game/Blueprint/GAS/GameplayAbility/Archer/ToxicInfestationArrow/Projectile/GE_ToxicInfestationArroe.GE_ToxicInfestationArroe_C" 0.0 (`AbilitySystemComponent.MakeEffectContext` _ownerasc)) (struct :`TagName` "Damage.AbilityTypeBonus") -0.7))
  (`AbilitySystemComponent.BP_ApplyGameplayEffectSpecToTarget` _ownerasc _returnvalue (`AbilitySystemBlueprintLibrary.GetAbilitySystemComponent` OtherActor)))

(event `self.BlueprintDelayedDestroy`
  (`parent.BlueprintDelayedDestroy`)
  (`ActorComponent.Deactivate` (`self.P_Trail_Poison`)))

(fn `UserConstructionScript`
  (`parent.UserConstructionScript`))
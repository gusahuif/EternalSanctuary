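; Arrow projectile for the Archer's Rapid Fire ability, layering GAS rune effects on the parent's collision handling.
; On collision, owner rune tags can add a Gale stack to the owner, apply Pierce vulnerability to the target, or let Hunt consume the target's Mark for damage scaled by its remaining duration.
; Every handled collision also applies the Rapid Fire cost effect to the owner; delayed destroy removes the arrow mesh.
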(event `self.ReceiveBeginPlay`
  (`parent.ReceiveBeginPlay`))

(event `self.HandleProjectileCollision`
  (params (OtherActor :type "Actor Object Reference") (OtherComp :type "PrimitiveComponent Object Reference") (bFromSweep :type Boolean) (SweepResult :type "HitResult Structure (by ref)"))
  (bind _returnvalue (`AbilitySystemBlueprintLibrary.GetAbilitySystemComponent` OtherActor))
  (bind _returnvalue_2 (`AbilitySystemBlueprintLibrary.GetAbilitySystemComponent` OtherActor))
  (bind _returnvalue_3 (`AbilitySystemBlueprintLibrary.GetAbilitySystemComponent` OtherActor))
  (bind _ownerasc (`self.OwnerASC`))
  (bind _ownerasc_2 (`self.OwnerASC`))
  (bind _ownerasc_3 (`self.OwnerASC`))
  (bind _ownerasc_4 (`self.OwnerASC`))
  (`parent.HandleProjectileCollision` OtherActor OtherComp bFromSweep SweepResult)
  (`|ExecutionSequence`
    (:`then_0`
      (if (`GameplayTagAssetInterface.HasMatchingGameplayTag` _ownerasc (struct :`TagName` "Rune.Archer.Gale"))
        (`AbilitySystemComponent.BP_ApplyGameplayEffectToSelf` _ownerasc "/Game/Blueprint/GAS/GameplayAbility/Archer/Base/RapidFire/Rune/Gale/GE_Gale_Stack.GE_Gale_Stack_C" 1.0 (`AbilitySystemComponent.MakeEffectContext` _ownerasc))))
    (:`then_1`
      (if (`GameplayTagAssetInterface.HasMatchingGameplayTag` _ownerasc_2 (struct :`TagName` "Rune.Archer.Pierce"))
        (`/Engine/EditorBlueprintResources/StandardMacros.IsValid` _returnvalue
          (:`Is Valid`
            (`AbilitySystemComponent.BP_ApplyGameplayEffectToTarget` _ownerasc_2 "/Game/Blueprint/GAS/GameplayAbility/Archer/Base/RapidFire/Rune/Pierce/GE_Pierce_Vulnerability.GE_Pierce_Vulnerability_C" _returnvalue 0.0 (`AbilitySystemComponent.MakeEffectContext` _ownerasc_2))
            (set `self.bHasRune` true)))))
    (:`then_2`
      (if (`GameplayTagAssetInterface.HasMatchingGameplayTag` (`self.OwnerASC`) (struct :`TagName` "Rune.Archer.Hunt"))
        (if (`GameplayTagAssetInterface.HasMatchingGameplayTag` _returnvalue_3 (struct :`TagName` "Debuff.Mark"))
          (bind _returnvalue_4 (`AbilitySystemComponent.GetActiveEffectsWithAllTags` _returnvalue_3 (struct :`GameplayTags` (struct :`(TagName` "Debuff.Mark")))))
          (if (> (`KismetArrayLibrary.Array_Length` _returnvalue_4) 0)
            (bind _returnvalue_5 (`AbilitySystemBlueprintLibrary.GetActiveGameplayEffectRemainingDuration` (`|GetArrayItem` _returnvalue_4)))
            (bind _returnvalue_6 (`AbilitySystemBlueprintLibrary.AssignTagSetByCallerMagnitude` (`AbilitySystemComponent.MakeOutgoingSpec` _ownerasc_3 "/Game/Blueprint/GAS/GameplayEffect/Combat/GE_Damage.GE_Damage_C" 1.0 (`AbilitySystemComponent.MakeEffectContext` _ownerasc_3)) (struct :`TagName` "Damage.AbilityTypeBonus") (- (* (`KismetMathLibrary.Conv_IntToDouble` (`KismetMathLibrary.FCeil` _returnvalue_5)) 0.3) 1.0)))
            (`AbilitySystemComponent.BP_ApplyGameplayEffectSpecToTarget` (`self.OwnerASC`) _returnvalue_6 _returnvalue_2)
            (`AbilitySystemComponent.RemoveActiveEffectsWithTags` _returnvalue_2 (struct :`GameplayTags` (struct :`(TagName` "Debuff.Mark"))))
            (set `self.bHasRune` true)))))
    (:`then_3`
      (`AbilitySystemComponent.BP_ApplyGameplayEffectToSelf` _ownerasc_4 "/Game/Blueprint/GAS/GameplayAbility/Archer/Base/RapidFire/GE/GE_Archer_Basic_Cost_RapidFire.GE_Archer_Basic_Cost_RapidFire_C" 0.0 (`AbilitySystemComponent.MakeEffectContext` _ownerasc_4)))))

(event `self.BlueprintDelayedDestroy`
  (`parent.BlueprintDelayedDestroy`)
  (`ActorComponent.K2_DestroyComponent` (`self.SM_Arrow_01`)))

(fn `UserConstructionScript`
  (`parent.UserConstructionScript`))
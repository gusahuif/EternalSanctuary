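; Demon Summoner ranged enemy character, built on a parent class and the Gameplay Ability System.
; On begin play it grants death, hit-react and ranged attack abilities, and randomly hides or shows its cape and halo independently for visual variation.
; The construction script makes the halo, weapon and cape skeletal meshes follow the main mesh as leader pose, so all pieces animate together.
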(event `self.ReceiveBeginPlay`
  (`parent.ReceiveBeginPlay`)
  (`SceneComponent.SetHiddenInGame` (`self.SK_DemonSummoner_Cape`) (`KismetMathLibrary.RandomBool`) false)
  (`SceneComponent.SetHiddenInGame` (`self.SK_DemonSummoner_Halo`) (`KismetMathLibrary.RandomBool`) false)
  (`AbilitySystemComponent.K2_GiveAbility` (`self.AbilitySystemComponent`) "/Game/Blueprint/Character/Enemy/Range/DemonSummoner/GA/GA_DemonSummoner_Dead.GA_DemonSummoner_Dead_C" 0 -1)
  (`AbilitySystemComponent.K2_GiveAbility` (`self.AbilitySystemComponent`) "/Game/Blueprint/Character/Enemy/Range/DemonSummoner/GA/GA_DemonSummoner_HitReact.GA_DemonSummoner_HitReact_C" 0 -1)
  (`AbilitySystemComponent.K2_GiveAbility` (`self.AbilitySystemComponent`) "/Game/Blueprint/Character/Enemy/Range/DemonSummoner/GA/GA_DemonSummoner_RangedAttack.GA_DemonSummoner_RangedAttack_C" 0 -1))

(fn `UserConstructionScript`
  (`parent.UserConstructionScript`)
  (`SkinnedMeshComponent.SetLeaderPoseComponent` (`self.SK_DemonSummoner_Halo`) (`self.Mesh`) false false)
  (`SkinnedMeshComponent.SetLeaderPoseComponent` (`self.SK_DemonSummoner_Weapon`) (`self.Mesh`) false false)
  (`SkinnedMeshComponent.SetLeaderPoseComponent` (`self.SK_DemonSummoner_Cape`) (`self.Mesh`) false false))
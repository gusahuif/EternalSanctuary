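; Humanoid scarab melee enemy character Blueprint that sets up its gameplay abilities.
; On BeginPlay it runs the parent logic, then grants melee attack, hit react and death abilities through the Gameplay Ability System.
; It adds no other logic: overlap and tick events are disabled, and the construction script only calls its parent.
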(event `self.ReceiveBeginPlay`
  (`parent.ReceiveBeginPlay`)
  (`AbilitySystemComponent.K2_GiveAbility` (`self.AbilitySystemComponent`) "/Game/Blueprint/Character/Enemy/Melee/HumanoidScarab/GA/GA_HumanoidScarab_MeleeAttack.GA_HumanoidScarab_MeleeAttack_C" 0 -1)
  (`AbilitySystemComponent.K2_GiveAbility` (`self.AbilitySystemComponent`) "/Game/Blueprint/Character/Enemy/Melee/HumanoidScarab/GA/GA_HumanoidScarab_HitReact.GA_HumanoidScarab_HitReact_C" 0 -1)
  (`AbilitySystemComponent.K2_GiveAbility` (`self.AbilitySystemComponent`) "/Game/Blueprint/Character/Enemy/Melee/HumanoidScarab/GA/GA_HumanoidScarab_Dead.GA_HumanoidScarab_Dead_C" 0 -1))

(fn `UserConstructionScript`
  (`parent.UserConstructionScript`))
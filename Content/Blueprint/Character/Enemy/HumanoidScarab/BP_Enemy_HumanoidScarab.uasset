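; BP_Enemy_HumanoidScarab is the Humanoid Scarab enemy character, with a text display of a Gameplay Ability System attribute.
; On BeginPlay it runs the parent logic, then writes the current attribute value from its AbilitySystemComponent to a TextRender.
; A persistent WaitForAttributeChanged async task updates that text on every change, avoiding Tick.
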(event `self.ReceiveBeginPlay`
  (`parent.ReceiveBeginPlay`)
  (bind (_asynctaskproxy _attribute _newvalue) (`AbilityAsync_WaitAttributeChanged.WaitForAttributeChanged` null (struct :`AttributeName` "Health" :`Attribute` "/Script/EternalSanctuary.ESAttributeSet:Health" :`AttributeOwner` "/Script/CoreUObject.Class'/Script/EternalSanctuary.ESAttributeSet'"))
    (:`then`
      (`TextRenderComponent.K2_SetText` (`self.TextRender`) (`KismetTextLibrary.Conv_DoubleToText` (`.ReturnValue` (`AbilitySystemBlueprintLibrary.GetFloatAttributeFromAbilitySystemComponent` (`self.AbilitySystemComponent`) (struct :`AttributeName` "Health" :`Attribute` "/Script/EternalSanctuary.ESAttributeSet:Health" :`AttributeOwner` "/Script/CoreUObject.Class'/Script/EternalSanctuary.ESAttributeSet'"))) "HalfToEven")))
    (:`Changed`
      (`TextRenderComponent.K2_SetText` (`self.TextRender`) (`KismetTextLibrary.Conv_DoubleToText` _newvalue "HalfToEven")))))

(fn `UserConstructionScript`
  (`parent.UserConstructionScript`))
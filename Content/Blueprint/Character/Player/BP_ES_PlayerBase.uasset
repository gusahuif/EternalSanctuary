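; Player base Blueprint built on the Gameplay Ability System that gives the character health regeneration.
; On BeginPlay it applies GE_HealthRegen to itself, passing percent and flat regen amounts as SetByCaller magnitudes.
; A hard-wired T key, apparently for testing, applies GE_Damage with an ability-type bonus magnitude to the first BP_EnemyBase found in the level.
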(event `self.ReceiveBeginPlay`
  (bind _abilitysystemcomponent (`self.AbilitySystemComponent`))
  (bind _returnvalue (`AbilitySystemBlueprintLibrary.AssignTagSetByCallerMagnitude` (`AbilitySystemComponent.MakeOutgoingSpec` _abilitysystemcomponent "/Game/Blueprint/GAS/GameplayEffect/Combat/GE_HealthRegen.GE_HealthRegen_C" 1.0 (`AbilitySystemComponent.MakeEffectContext` _abilitysystemcomponent)) (struct :`TagName` "Regen.HealthPercent") 0.02))
  (bind _returnvalue_2 (`AbilitySystemBlueprintLibrary.AssignTagSetByCallerMagnitude` _returnvalue (struct :`TagName` "Regen.FlatHealth") 5.0))
  (`AbilitySystemComponent.BP_ApplyGameplayEffectSpecToSelf` (`self.AbilitySystemComponent`) _returnvalue_2))

(event `Key|T`
  (params (Key :type "Key Structure"))
  (bind _abilitysystemcomponent (`self.AbilitySystemComponent`))
  (:`Pressed`
    (bind _outactors (`GameplayStatics.GetAllActorsOfClass` "/Game/Blueprint/Character/Enemy/BP_EnemyBase.BP_EnemyBase_C"))
    (bind _returnvalue (`AbilitySystemBlueprintLibrary.AssignTagSetByCallerMagnitude` (`AbilitySystemComponent.MakeOutgoingSpec` _abilitysystemcomponent "/Game/Blueprint/GAS/GameplayEffect/Combat/GE_Damage.GE_Damage_C" 1.0 (`AbilitySystemComponent.MakeEffectContext` _abilitysystemcomponent)) (struct :`TagName` "Damage.AbilityTypeBonus") 1.0))
    (`AbilitySystemComponent.BP_ApplyGameplayEffectSpecToTarget` _abilitysystemcomponent _returnvalue (`AbilitySystemBlueprintLibrary.GetAbilitySystemComponent` (`|GetArrayItem` _outactors)))))

(fn `UserConstructionScript`)
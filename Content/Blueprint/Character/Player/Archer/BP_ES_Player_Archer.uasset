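; Player character Blueprint for the Archer, set up through the Gameplay Ability System.
; On BeginPlay, after the parent logic, it grants the Rapid Fire ability to the basic ability slot and applies the Gale rune gameplay effect to itself.
; The construction script only calls the parent, and the overlap and tick events are unused.
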(event `self.ReceiveBeginPlay`
  (bind _abilitysystemcomponent (`self.AbilitySystemComponent`))
  (`parent.ReceiveBeginPlay`)
  (`ESAbilitySystemComponent.GiveAbilityToSlot` (`self.AbilitySystemComponent`) (struct :`TagName` "Ability.Slot.Basic") "/Game/Blueprint/GAS/GameplayAbility/Archer/Base/RapidFire/GA_Archer_Basic_RapidFire.GA_Archer_Basic_RapidFire_C" 1)
  (`AbilitySystemComponent.BP_ApplyGameplayEffectToSelf` _abilitysystemcomponent "/Game/Blueprint/GAS/GameplayAbility/Archer/Base/RapidFire/Rune/Gale/GE_Rune_Gale.GE_Rune_Gale_C" 1.0 (`AbilitySystemComponent.MakeEffectContext` _abilitysystemcomponent)))

(fn `UserConstructionScript`
  (`parent.UserConstructionScript`))
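; Fireball projectile Blueprint that relies on its parent class for nearly all of its behavior.
; On BeginPlay it runs the parent logic, then prints the OwnerActor name as debug output.
; Its delayed-destroy event calls the parent, then deactivates the PProjectileFire component.
; The overlap and Tick events are disabled stubs, and the construction script only calls its parent.
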(event `self.ReceiveBeginPlay`
  (`parent.ReceiveBeginPlay`)
  (`KismetSystemLibrary.PrintString` (`KismetStringLibrary.Concat_StrStr` "OwnerActor=" (`KismetSystemLibrary.GetDisplayName` (`self.OwnerActor`)))))

(event `self.BlueprintDelayedDestroy`
  (`parent.BlueprintDelayedDestroy`)
  (`ActorComponent.Deactivate` (`self.P_Projectile_Fire`)))

(fn `UserConstructionScript`
  (`parent.UserConstructionScript`))
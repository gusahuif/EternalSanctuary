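; BP_PickupEquip is a dropped equipment pickup that scatters out from its spawn point and waits for player interaction.
; It picks ribbon and landed Niagara effects by item quality, then a randomly timed Timeline arcs it to a random nearby offset at the player's foot height.
; On landing it swaps effects and enables overlaps, which toggle a quality-colored name prompt on the HUD.
; The interaction trigger calls OnInteract with the player pawn.
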(event `self.ReceiveBeginPlay`
  (bind _returnvalue (`GameplayStatics.GetPlayerCharacter` 0))
  (bind _spawnlocation (`self.SpawnLocation`))
  (`KismetSystemLibrary.DelayUntilNextFrame`)
  (`NiagaraComponent.SetAsset` (`self.VFX_Ribbon`) (select `EESItemQuality` (`ESItemBase.Quality` (`self.SavedEquipItem`)) :`Normal` "/Game/Asset/VFX/sA_ItemDropFx/Fx/NS_Normal_Ribbon.NS_Normal_Ribbon" :`Rare` "/Game/Asset/VFX/sA_ItemDropFx/Fx/NS_Rare_Ribbon.NS_Rare_Ribbon" :`Legendary` "/Game/Asset/VFX/sA_ItemDropFx/Fx/NS_Legendary_Ribbon.NS_Legendary_Ribbon" :!type "NiagaraSystem Object Reference") true)
  (`NiagaraComponent.SetAsset` (`self.VFX_System`) (select `EESItemQuality` (`ESItemBase.Quality` (`self.SavedEquipItem`)) :`Normal` "/Game/Asset/VFX/sA_ItemDropFx/Fx/NS_Normal_System.NS_Normal_System" :`Rare` "/Game/Asset/VFX/sA_ItemDropFx/Fx/NS_Rare_System.NS_Rare_System" :`Legendary` "/Game/Asset/VFX/sA_ItemDropFx/Fx/NS_Legendary_System.NS_Legendary_System" :!type "NiagaraSystem Object Reference") true)
  (set `self.ZHight` (+ (- (.z (`self.K2_GetActorLocation` _returnvalue)) (`.OutHalfHeight` (`CapsuleComponent.GetScaledCapsuleSize` (`Character.CapsuleComponent` _returnvalue)))) 5.0))
  (set `self.RandomOffset` (* (`KismetMathLibrary.GetForwardVector` (`KismetMathLibrary.MakeRotator` 0.0 0.0 (`KismetMathLibrary.RandomFloatInRange` -180.0 180.0))) (`KismetMathLibrary.Conv_DoubleToVector` (`KismetMathLibrary.RandomFloatInRange` 100.0 200.0))))
  (set `self.SpawnLocation` (`self.K2_GetActorLocation`))
  (`TimelineComponent.SetPlayRate` (`self.Timeline`) (/ 1.0 (`KismetMathLibrary.RandomFloatInRange` 0.3 0.5)))
  (bind (_direction _z _alpha) (`Timeline|Timeline` :!via `PlayFromStart`)
    (:`Update`
      (`self.K2_SetActorLocation` (`KismetMathLibrary.MakeVector` (.x (`KismetMathLibrary.VLerp` _spawnlocation (+ _spawnlocation (`self.RandomOffset`)) _alpha)) (.y (`KismetMathLibrary.VLerp` _spawnlocation (+ _spawnlocation (`self.RandomOffset`)) _alpha)) (+ (`self.ZHight`) (* _z 100.0)))))
    (:`Finished`
      (`ActorComponent.Deactivate` (`self.VFX_Ribbon`))
      (`ActorComponent.Activate` (`self.VFX_System`) true)
      (set `PrimitiveComponent.bGenerateOverlapEvents` true (`self.CollisionSphere`))
      (`self.K2_AddActorLocalOffset` (0.0 0.0 1.0)))))

(event `/Game/Blueprint/Common/Interaction/Interface/BPI_Interaction.OnInteractionTrigger`
  (`self.OnInteract` (`GameplayStatics.GetPlayerPawn` 0)))

(event `self.CollisionSphere.OnComponentBeginOverlap`
  (params (OverlappedComponent :type "PrimitiveComponent Object Reference") (OtherActor :type "Actor Object Reference") (OtherComp :type "PrimitiveComponent Object Reference") (OtherBodyIndex :type Integer) (bFromSweep :type Boolean) (SweepResult :type "HitResult Structure (by ref)"))
  (if (== OtherActor (`GameplayStatics.GetPlayerPawn` 0))
    (`/Game/Blueprint/Core/BP_ES_HUD.ChangeInteractionVisibility` (`/Game/Blueprint/Item/Lib/BFL_Item.GetESHUD`) true (`ESItemBase.Name` (`self.SavedEquipItem`)) (`ESItemBase.GetQualityColor` (`self.SavedEquipItem`)) self)))

(event `self.CollisionSphere.OnComponentEndOverlap`
  (params (OverlappedComponent :type "PrimitiveComponent Object Reference") (OtherActor :type "Actor Object Reference") (OtherComp :type "PrimitiveComponent Object Reference") (OtherBodyIndex :type Integer))
  (if (== OtherActor (`GameplayStatics.GetPlayerPawn` 0))
    (`/Game/Blueprint/Core/BP_ES_HUD.ChangeInteractionVisibility` (`/Game/Blueprint/Item/Lib/BFL_Item.GetESHUD`) false "" (struct :`R` 1.0 :`G` 1.0 :`B` 1.0 :`A` 1.0) self)))

(fn `UserConstructionScript`)
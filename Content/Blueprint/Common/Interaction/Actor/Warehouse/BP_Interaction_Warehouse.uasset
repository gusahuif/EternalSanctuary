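; BP_Interaction_Warehouse is an interaction actor that gives access to the warehouse UI panel.
; TriggerEvent calls its parent, then toggles the panel through the ES HUD, closing it if the cached warehouse panel is visible and opening it otherwise.
; FinishEvent calls its parent, then closes the panel.
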(event `self.TriggerEvent`
  (`parent.TriggerEvent`)
  (if (`Widget.IsVisible` (`/Game/Blueprint/Core/BP_ES_HUD.CachedWarehousePanel` (`/Game/Blueprint/Item/Lib/BFL_Item.GetESHUD`)))
    (`/Game/Blueprint/Core/BP_ES_HUD.CloseWarehousePanel` (`/Game/Blueprint/Item/Lib/BFL_Item.GetESHUD`))
    (else
      (`/Game/Blueprint/Core/BP_ES_HUD.OpenWarehousePanel` (`/Game/Blueprint/Item/Lib/BFL_Item.GetESHUD`)))))

(event `self.FinishEvent`
  (`parent.FinishEvent`)
  (`/Game/Blueprint/Core/BP_ES_HUD.CloseWarehousePanel` (`/Game/Blueprint/Item/Lib/BFL_Item.GetESHUD`)))

(fn `UserConstructionScript`
  (`parent.UserConstructionScript`))
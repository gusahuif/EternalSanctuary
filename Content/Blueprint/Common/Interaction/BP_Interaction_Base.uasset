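; Base interaction actor that shows a HUD prompt while the player pawn is inside its trigger sphere.
; Sphere overlaps register or remove the actor on the ES HUD through ChangeInteractionVisibility, using its UI text and color.
; OnInteractionTrigger forwards to TriggerEvent, and leaving the sphere calls FinishEvent whether or not it was triggered.
; Both events are empty here, serving as hooks for child interaction Blueprints.
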(event `self.Sphere.OnComponentBeginOverlap`
  (params (OverlappedComponent :type "PrimitiveComponent Object Reference") (OtherActor :type "Actor Object Reference") (OtherComp :type "PrimitiveComponent Object Reference") (OtherBodyIndex :type Integer) (bFromSweep :type Boolean) (SweepResult :type "HitResult Structure (by ref)"))
  (if (== OtherActor (`GameplayStatics.GetPlayerPawn` 0))
    (`/Game/Blueprint/Core/BP_ES_HUD.ChangeInteractionVisibility` (`/Game/Blueprint/Item/Lib/BFL_Item.GetESHUD`) true (`self.UIText`) (`self.UIColor`) self)))

(event `self.Sphere.OnComponentEndOverlap`
  (params (OverlappedComponent :type "PrimitiveComponent Object Reference") (OtherActor :type "Actor Object Reference") (OtherComp :type "PrimitiveComponent Object Reference") (OtherBodyIndex :type Integer))
  (if (== OtherActor (`GameplayStatics.GetPlayerPawn` 0))
    (`/Game/Blueprint/Core/BP_ES_HUD.ChangeInteractionVisibility` (`/Game/Blueprint/Item/Lib/BFL_Item.GetESHUD`) false "" (struct :`R` 1.0 :`G` 1.0 :`B` 1.0 :`A` 1.0) self)
    (`self.FinishEvent`)))

(event `TriggerEvent`)

(event `FinishEvent`)

(event `/Game/Blueprint/Common/Interaction/Interface/BPI_Interaction.OnInteractionTrigger`
  (`self.TriggerEvent`))

(fn `UserConstructionScript`)